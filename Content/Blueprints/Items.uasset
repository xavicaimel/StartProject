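; Items is a collectible pickup that spins in place and adds to the player's item count when touched.
; Each tick it applies a swept local rotation from the Rotador variable.
; On any actor overlap it destroys itself, then casts player 0's character to FirstPersonCharacter, increments its Items counter and prints the total, without checking which actor overlapped.
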(event `self.ReceiveTick`
  (params (DeltaSeconds :type "Float (single-precision)"))
  (`self.K2_AddActorLocalRotation` (`self.Rotador`) true))

(event `self.ReceiveActorBeginOverlap`
  (params (OtherActor :type "Actor Object Reference"))
  (`self.K2_DestroyActor`)
  (bind _asfirst_person_character (cast `/Game/FirstPersonBP/Blueprints/FirstPersonCharacter` (`GameplayStatics.GetPlayerCharacter` 0)))
  (bind _output_get (set `/Game/FirstPersonBP/Blueprints/FirstPersonCharacter.Items` (+ (`/Game/FirstPersonBP/Blueprints/FirstPersonCharacter.Items` _asfirst_person_character) 1) _asfirst_person_character))
  (`KismetSystemLibrary.PrintString` (`KismetStringLibrary.Conv_IntToString` _output_get)))

(fn `UserConstructionScript`)